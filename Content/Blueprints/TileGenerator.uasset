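; Actor that procedurally builds a tiled, box-shaped room with floor, ceiling, perimeter walls and lights at BeginPlay.
; The construction script assigns meshes to the Floor and Wall instanced components, and GenerateMap walks the grid calling per-piece placement functions.
; Ceiling tiles reuse the Floor component, and SetMaterial receives each instance index as its material slot.
; Every LightFrequency tiles, it adds a ceiling fixture instance and a configured point light with an IES profile.
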(event EventBeginPlay
  (CallFunction|GenerateMap))

(event EventActorBeginOverlap
  (params (OtherActor :type Actor%20Object%20Reference)))

(event EventTick
  (params (DeltaSeconds :type Float%20%28single-precision%29)))

(fn ConstructionScript
  (Components|StaticMesh|SetStaticMesh (Variables|Default|GetFloor) (Variables|Materials|GetFloorMesh))
  (Components|StaticMesh|SetStaticMesh (Variables|Default|GetWall) (Variables|Materials|GetWallMesh)))

(fn GenerateMap
  (bind _lightfrequency (Variables|Lighting|GetLightFrequency))
  (for _index (range 0 (Utilities|MaxY))
    (CallFunction|PlaceLeftWallat (Utilities|MaxX) _index)
    (CallFunction|PlaceRightWallat 0 _index)
    (for _index_2 (range 0 (Utilities|MaxX))
      (CallFunction|PlaceFloorat _index_2 _index)
      (CallFunction|PlaceCeilingat _index_2 _index)
      (if (and (== (Math|Integer|%(Integer) _index_2 _lightfrequency) 0) (== (Math|Integer|%(Integer) _index _lightfrequency) 0))
        (CallFunction|PlaceLightat _index_2 _index))))
  (for _index_3 (range 0 (Utilities|MaxX))
    (CallFunction|PlaceFrontWallat _index_3 (Utilities|MaxY))
    (CallFunction|PlaceBackWallat _index_3))
  (return))

(fn PlaceFloorat
  (params (x :type Integer :default 0) (y :type Integer :default 0))
  (bind _tilesize (Variables|Default|GetTileSize))
  (bind _floor (Variables|Default|GetFloor))
  (bind _returnvalue (Components|InstancedStaticMesh|AddInstance _floor (Math|Conversions|ToTransform(Vector) (Math|Vector|MakeVector (Math|Conversions|ToFloat(Integer) (* x _tilesize)) (Math|Conversions|ToFloat(Integer) (* _tilesize y)) 0.0))))
  (Rendering|Material|SetMaterial _floor _returnvalue (Variables|Materials|GetFloorMaterial))
  (return))

(fn PlaceLeftWallat
  (params (x :type Integer :default 0) (y :type Integer :default 0))
  (bind _tilesize (Variables|Default|GetTileSize))
  (bind _wall (Variables|Default|GetWall))
  (for _index (range 0 (Utilities|MaxZ))
    (bind _returnvalue (Components|InstancedStaticMesh|AddInstance _wall (Math|Transform|MakeTransform (Math|Vector|MakeVector (Math|Conversions|ToFloat(Integer) (+ (* x _tilesize) _tilesize)) (Math|Conversions|ToFloat(Integer) (* _tilesize y)) (Math|Conversions|ToFloat(Integer) (* _index (Variables|Default|GetTileSize)))) "0,90.000000, 0")))
    (Rendering|Material|SetMaterial _wall _returnvalue (Variables|Materials|GetWallMaterial))
    (return)))

(fn PlaceRightWallat
  (params (x :type Integer :default 0) (y :type Integer :default 0))
  (bind _tilesize (Variables|Default|GetTileSize))
  (bind _wall (Variables|Default|GetWall))
  (for _index (range 0 (Utilities|MaxZ))
    (bind _returnvalue (Components|InstancedStaticMesh|AddInstance _wall (Math|Transform|MakeTransform (Math|Vector|MakeVector (Math|Conversions|ToFloat(Integer) (* x _tilesize)) (Math|Conversions|ToFloat(Integer) (+ _tilesize (* _tilesize y))) (Math|Conversions|ToFloat(Integer) (* _index (Variables|Default|GetTileSize)))) "0,-90.000000, 0")))
    (Rendering|Material|SetMaterial _wall _returnvalue (Variables|Materials|GetWallMaterial))
    (return)))

(fn PlaceFrontWallat
  (params (x :type Integer :default 0) (y :type Integer :default 0))
  (bind _tilesize (Variables|Default|GetTileSize))
  (bind _wall (Variables|Default|GetWall))
  (for _index (range 0 (Utilities|MaxZ))
    (bind _returnvalue (Components|InstancedStaticMesh|AddInstance _wall (Math|Transform|MakeTransform (Math|Vector|MakeVector (Math|Conversions|ToFloat(Integer) (+ (* x _tilesize) _tilesize)) (Math|Conversions|ToFloat(Integer) (+ _tilesize (* _tilesize y))) (Math|Conversions|ToFloat(Integer) (* _index (Variables|Default|GetTileSize)))) "0,180.000000, 0")))
    (Rendering|Material|SetMaterial _wall _returnvalue (Variables|Materials|GetWallMaterial))
    (return)))

(fn PlaceBackWallat
  (params (x :type Integer) (y :type Integer))
  (bind _wall (Variables|Default|GetWall))
  (bind _tilesize (Variables|Default|GetTileSize))
  (for _index (range 0 (Utilities|MaxZ))
    (bind _returnvalue (Components|InstancedStaticMesh|AddInstance _wall (Math|Conversions|ToTransform(Vector) (Math|Vector|MakeVector (Math|Conversions|ToFloat(Integer) (* x _tilesize)) (Math|Conversions|ToFloat(Integer) (* _tilesize y)) (Math|Conversions|ToFloat(Integer) (* _index (Variables|Default|GetTileSize)))))))
    (Rendering|Material|SetMaterial _wall _returnvalue (Variables|Materials|GetWallMaterial))
    (return)))

(fn PlaceLightat
  (params (x :type Integer :default 0) (y :type Integer :default 0))
  (bind _lightheight (Variables|Lighting|GetLightHeight))
  (bind _tilesize (Variables|Default|GetTileSize))
  (bind _returnvalue (/ _tilesize 2))
  (bind _returnvalue_2 (* _tilesize y))
  (bind _returnvalue_3 (* x _tilesize))
  (bind _returnvalue_4 (Math|Conversions|ToFloat(Integer) _returnvalue_3))
  (bind _returnvalue_5 (Math|Conversions|ToFloat(Integer) _returnvalue_2))
  (bind _returnvalue_6 (Math|Conversions|ToFloat(Integer) _returnvalue))
  (bind _returnvalue_7 (Math|Vector|MakeVector _returnvalue_4 _returnvalue_5 _lightheight))
  (bind _returnvalue_8 (Math|Vector|MakeVector _returnvalue_6 _returnvalue_6 0.0))
  (bind _returnvalue_9 (+ _returnvalue_7 _returnvalue_8))
  (Components|InstancedStaticMesh|AddInstance (Variables|Default|GetCeiling%20Light) (Math|Conversions|ToTransform(Vector) (+ "-75.000000,-25.000000,0.000000" _returnvalue_9)))
  (bind _returnvalue_10 (AddComponent|AddPointLightComponent false (Math|Conversions|ToTransform(Vector) _returnvalue_9)))
  (Rendering|Components|Light|SetIntensity _returnvalue_10 (Variables|Lighting|GetLightIntensity))
  (Rendering|Components|Light|SetLightColor _returnvalue_10 "(R=0.865000,G=0.876232,B=1.000000,A=1.000000)")
  (Rendering|Lighting|SetAttenuationRadius _returnvalue_10 (Variables|Lighting|GetLightAttenuationRadius))
  (Rendering|Components|Light|SetCastShadows _returnvalue_10 (Variables|Lighting|GetLightCastsShadows))
  (Class|LightComponent|SetIESTexture _returnvalue_10 "/Game/Materials/2FSL4_60L_LP835.2FSL4_60L_LP835")
  (Transformation|SetRelativeRotation _returnvalue_10 "-90.000000,90.000000,0.000000" false)
  (return))

(fn PlaceCeilingat
  (params (X :type Integer :default 0) (Y :type Integer :default 0))
  (bind _tilesize (Variables|Default|GetTileSize))
  (bind _floor (Variables|Default|GetFloor))
  (bind _returnvalue (Components|InstancedStaticMesh|AddInstance _floor (Math|Conversions|ToTransform(Vector) (Math|Vector|MakeVector (Math|Conversions|ToFloat(Integer) (* X _tilesize)) (Math|Conversions|ToFloat(Integer) (* _tilesize Y)) (Math|Conversions|ToFloat(Integer) (+ (* _tilesize (Variables|Default|GetHeight)) (Variables|Default|GetTileThickness)))))))
  (Rendering|Material|SetMaterial _floor _returnvalue (Variables|Materials|GetCeilingMaterial)))
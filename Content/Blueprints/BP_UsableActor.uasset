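; BP_UsableActor is a pickup actor that a character can focus on and use to add it as an item.
; BeginFocus shows its DisplayName as the character's action text and turns custom depth rendering off, while EndFocus hides the text and turns it back on.
; OnUsed ends focus, passes itself to the character's AddItem, then hides itself and moves to the world origin instead of being destroyed.
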(event EventBeginPlay)

(event EventActorBeginOverlap
  (params (OtherActor :type Actor%20Object%20Reference)))

(event EventTick
  (params (DeltaSeconds :type Float%20%28single-precision%29)))

(fn ConstructionScript)

(fn BeginFocus
  (params (Character :type Character%20BP%20Object%20Reference))
  (Rendering|SetRenderCustomDepth false)
  (Variables|/Game/Blueprints/CharacterBP.CharacterBP_C|SetAction%20Text Character (Variables|Default|GetDisplayName))
  (Variables|/Game/Blueprints/CharacterBP.CharacterBP_C|SetShow%20Action%20Text Character true)
  (return false))

(fn EndFocus
  (params (Character :type Character%20BP%20Object%20Reference))
  (Rendering|SetRenderCustomDepth true)
  (Variables|/Game/Blueprints/CharacterBP.CharacterBP_C|SetShow%20Action%20Text Character false)
  (return false))

(fn OnUsed
  (params (Character :type Character%20BP%20Object%20Reference))
  (CallFunction|EndFocus Character)
  (Default|AddItem Character self)
  (Rendering|SetActorHiddenInGame true)
  (Transformation|SetActorTransform (Math|Transform|MakeTransform "0, 0, 0"))
  (return false))
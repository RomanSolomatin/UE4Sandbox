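; Powered two-door airlock that opens when a pawn enters its sensor or toggles on interact, unless bolted.
; The DoorDriver timeline slides and squashes both doors, then closes them after opening, with an optional retriggerable delay.
; Swept movement detects obstructions, either calling reopen under safety or damaging the blocker and pushing through.
; Electrified doors damage pawns that hit them, with brief sparks and sound.
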(event OnComponentHit(AirlockLeft)
  (params (OtherActor :type Actor%20Object%20Reference) (OtherComp :type Primitive%20Component%20Object%20Reference) (NormalImpulse :type Vector :default "0, 0, 0") (Hit :type Hit%20Result%20Structure%20%28by%20ref%29))
  ;[1 1 1] AirlockSafety/Damage
  (bind _aspawn (Utilities|Casting|CastToPawn OtherActor))
  (if (Variables|Default|GetbIsElectrified)
    (Game|Damage|ApplyDamage _aspawn 5.0 0 0)
    (Components|Activation|Activate (Variables|Default|GetAirlockSparks) false)
    (if (Audio|Components|Audio|IsPlaying (Variables|Default|GetAirlockSparksSound))
      _
      (else
        (Audio|Components|Audio|Play (Variables|Default|GetAirlockSparksSound) 0.0)))
    (Utilities|FlowControl|RetriggerableDelay 0.5)
    (Audio|Components|Audio|Stop (Variables|Default|GetAirlockSparksSound))
    (Components|Activation|Deactivate (Variables|Default|GetAirlockSparks))))

(event OnComponentHit(AirlockRight)
  (params (OtherActor :type Actor%20Object%20Reference) (OtherComp :type Primitive%20Component%20Object%20Reference) (NormalImpulse :type Vector :default "0, 0, 0") (Hit :type Hit%20Result%20Structure%20%28by%20ref%29))
  ;[1 1 1] AirlockSafety/Damage
  (bind _aspawn (Utilities|Casting|CastToPawn OtherActor))
  (if (Variables|Default|GetbIsElectrified)
    (Game|Damage|ApplyDamage _aspawn 5.0 0 0)
    (Components|Activation|Activate (Variables|Default|GetAirlockSparks) false)
    (if (Audio|Components|Audio|IsPlaying (Variables|Default|GetAirlockSparksSound))
      _
      (else
        (Audio|Components|Audio|Play (Variables|Default|GetAirlockSparksSound) 0.0)))
    (Utilities|FlowControl|RetriggerableDelay 0.5)
    (Audio|Components|Audio|Stop (Variables|Default|GetAirlockSparksSound))
    (Components|Activation|Deactivate (Variables|Default|GetAirlockSparks))))

(event OnComponentBeginOverlap(AirlockCollision)
  (params (OtherActor :type Actor%20Object%20Reference) (OtherComp :type Primitive%20Component%20Object%20Reference) (OtherBodyIndex :type Integer) (bFromSweep :type Boolean) (SweepResult :type Hit%20Result%20Structure%20%28by%20ref%29))
  ;[1 1 1] AirlockSensor
  (Utilities|Casting|CastToPawn OtherActor)
  (if (Variables|Default|GetbHasPower)
    (CallFunction|AirlockOpen)))

(event Custom|AirlockOpenEvent
  ;[1 1 1] AirlockOpen/Close
  (if (not (Variables|Default|GetbIsBolted))
    (Variables|Default|SetbAirlockIsOpen true)
    (Audio|Components|Audio|Play (Variables|Default|GetAirlockSound) 0.0)
    (bind (_direction _driver) (Timeline|DoorDriver Play)
      (:Update
        (CallFunction|SetAirlockPosition _driver))
      (:Finished
        ;;[1 1 1] AirlockCloseDelay
        (Audio|Components|Audio|Stop (Variables|Default|GetAirlockSound))
        (if (Utilities|Enum|Equal(Enum) _direction "Forward")
          (if (Variables|Default|GetbDelayEnabled)
            (Utilities|FlowControl|RetriggerableDelay (Variables|Default|GetCloseDelay)))
          (CallFunction|AirlockClose))))))

(event Custom|AirlockCloseEvent
  ;[1 1 1] AirlockOpen/Close
  (if (not (Variables|Default|GetbIsBolted))
    (Variables|Default|SetbAirlockIsOpen false)
    (Audio|Components|Audio|Play (Variables|Default|GetAirlockSound) 0.0)
    (bind (_direction _driver) (Timeline|DoorDriver Reverse)
      (:Update
        (CallFunction|SetAirlockPosition _driver))
      (:Finished
        ;;[1 1 1] AirlockCloseDelay
        (Audio|Components|Audio|Stop (Variables|Default|GetAirlockSound))
        (if (Utilities|Enum|Equal(Enum) _direction "Forward")
          (if (Variables|Default|GetbDelayEnabled)
            (Utilities|FlowControl|RetriggerableDelay (Variables|Default|GetCloseDelay)))
          (CallFunction|AirlockClose))))))

(event EventOnInteract
  (params (Component :type Primitive%20Component%20Object%20Reference) (Item :type Integer))
  ;[1 1 1] Airlock Interaction
  (CallFunction|AirlockToggle))

(fn ConstructionScript)

(fn AirlockOpen
  (if (not (Variables|Default|GetbAirlockIsOpen))
    (CallFunction|AirlockOpenEvent)))

(fn AirlockClose
  (if (Variables|Default|GetbAirlockIsOpen)
    (CallFunction|AirlockCloseEvent)))

(fn AirlockToggle
  (if (Variables|Default|GetbAirlockIsOpen)
    (CallFunction|AirlockCloseEvent)
    (else
      (CallFunction|AirlockOpenEvent))))

(fn SetAirlockPosition
  (params (Alpha :type Float%20%28single-precision%29))
  (LocalVariables|SetDoorPos Alpha)
  (Utilities|FlowControl|Sequence
    (:then_0
      ;[1 1 1] LeftDoor
      (bind _output_get (LocalVariables|SetDoorTransform (Math|Transform|Lerp(Transform) (Utilities|ZeroTransform) (Math|Transform|MakeTransform "36.000000, 0, 0" "0, 0, 0" "0.100000,1,1") (LocalVariables|GetDoorPos))))
      (bind _sweephitresult (Transformation|SetRelativeTransform (Variables|Default|GetAirlockLeft) _output_get true))
      (LocalVariables|SetDoorHitResult _sweephitresult)
      (if (.bBlockingHit (Collision|BreakHitResult _sweephitresult))
        (if (Variables|Default|GetbSafetyEnabled)
          (CallFunction|AirlockOpen)
          (else
            (Game|Damage|ApplyPointDamage (.HitActor (Collision|BreakHitResult _sweephitresult)) 5.0 (.ImpactNormal (Collision|BreakHitResult _sweephitresult)) (LocalVariables|GetDoorHitResult) 0 self)
            (Transformation|SetRelativeTransform (Variables|Default|GetAirlockLeft) (LocalVariables|GetDoorTransform) false)))))
    (:then_1
      ;[1 1 1] RightDoor
      (bind _output_get_2 (LocalVariables|SetDoorTransform (Math|Transform|Lerp(Transform) (Utilities|ZeroTransform) (Math|Transform|MakeTransform "233.000000,0.000000, 0" "0, 0, 0" "0.100000,1,1") (LocalVariables|GetDoorPos))))
      (bind _sweephitresult_2 (Transformation|SetRelativeTransform (Variables|Default|GetAirlockRight) _output_get_2 true))
      (LocalVariables|SetDoorHitResult _sweephitresult_2)
      (if (.bBlockingHit (Collision|BreakHitResult _sweephitresult_2))
        (if (Variables|Default|GetbSafetyEnabled)
          (CallFunction|AirlockOpen)
          (else
            (Game|Damage|ApplyPointDamage (.HitActor (Collision|BreakHitResult _sweephitresult_2)) 5.0 (.ImpactNormal (Collision|BreakHitResult _sweephitresult_2)) (LocalVariables|GetDoorHitResult) 0 self)
            (Transformation|SetRelativeTransform (Variables|Default|GetAirlockRight) (LocalVariables|GetDoorTransform) false)))))))